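; Player controller for a turn-based sushi game, handling turn transitions, game start and touch input.
; Turn start shows the controlled player's hand; turn end updates all players' plates, refreshes and hides the hand, then rotates the Giratutti one plate step.
; Key 1 on authority makes the game mode locate players and start the game, then positions Giratutti plates.
; Touch release calls TapFocusable and prints the result.
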(event `self.ReceiveBeginPlay`)

(event `self.ReceiveTick`
  (params (DeltaSeconds :type "Float (single-precision)")))

(event `self.StartTurnBP`
  (`KismetSystemLibrary.PrintString` "START TURN" true true (struct :`G` 1.0 :`B` 0.596078 :`A` 1.0) 1.0)
  (bind _assushi_player_bp (cast `/Game/Actors/Player/SushiPlayer_BP` (`self.K2_GetPawn`)))
  (`SceneComponent.SetVisibility` (`/Game/Actors/Player/SushiPlayer_BP.SushisHand` _assushi_player_bp) true true))

(event `self.FinishTurnBP`
  (`KismetSystemLibrary.PrintString` "END TURN" true true (struct :`G` 1.0 :`B` 0.596078 :`A` 1.0) 1.0)
  ;[1 1 1] Update plate
  (bind _outactors (`GameplayStatics.GetAllActorsOfClass` "/Game/Actors/Player/SushiPlayer_BP.SushiPlayer_BP_C"))
  (for _array_element _outactors
    (`/Game/Actors/Player/SushiPlayer_BP.UpdatePlate` _array_element))
  ;[1 1 1] Update hand
  (bind _assushi_player_bp (cast `/Game/Actors/Player/SushiPlayer_BP` (`self.K2_GetPawn`)))
  (`/Game/Actors/Player/SushiPlayer_BP.UpdateHand` _assushi_player_bp)
  (`SceneComponent.SetVisibility` (`/Game/Actors/Player/SushiPlayer_BP.SushisHand` _assushi_player_bp) false true)
  ;[1 1 1] Rotate giratutti
  (bind _assushi_game_state_base (cast `SushiGameStateBase` (`GameplayStatics.GetGameState`)))
  (bind _returnvalue (`GameplayStatics.GetActorOfClass` "/Game/Actors/Giratutti.Giratutti_C"))
  (`/Game/Actors/Giratutti.Rotate` _returnvalue (/ 360.0 (`KismetMathLibrary.Conv_IntToDouble` (`KismetArrayLibrary.Array_Length` (`SushiGameStateBase.Plates` _assushi_game_state_base))))))

(event `Key|One`
  (params (Key :type "Key Structure"))
  (:`Pressed`
    (`/Engine/EditorBlueprintResources/ActorMacros.Switch Has Authority`
      (:`Authority`
        (`KismetSystemLibrary.PrintString` "Locating players and starting game")
        (`KismetSystemLibrary.Delay` 1.0)
        (bind _assushi_game_mode_bp (cast `/Game/SushiGameMode_BP` (`GameplayStatics.GetGameMode`)))
        (`/Game/SushiGameMode_BP.LocatePlayers` _assushi_game_mode_bp)
        (`SushiGameGameMode.InitSushiGame` _assushi_game_mode_bp)
        (bind _returnvalue (`GameplayStatics.GetActorOfClass` "/Game/Actors/Giratutti.Giratutti_C"))
        (`/Game/Actors/Giratutti.LocateGiratuttiPlates` _returnvalue)))))

(event `InputTouch`
  (params (Location :type "Vector Structure") (FingerIndex :type "ETouchIndex Enum"))
  (:`Released`
    (bind _returnvalue (`self.TapFocusable` self (`KismetMathLibrary.Conv_VectorToVector2D` Location)))
    (`KismetSystemLibrary.PrintString` (`KismetSystemLibrary.GetDisplayName` _returnvalue))))

(fn `UserConstructionScript`)
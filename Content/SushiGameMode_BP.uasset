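; Sushi game mode that arranges all players evenly in a circle around the world origin.
; LocatePlayers runs on the authority and steps an accumulated yaw by 360 divided by the player count for each SushiPlayer_BP.
; A PlayerStart supplies the circle's radius, from its horizontal distance to the origin, and its height.
; Each player is moved to its slot and rotated to face the centre.
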(event `LocatePlayers`
  (`/Engine/EditorBlueprintResources/ActorMacros.Switch Has Authority`
    (:`Authority`
      (bind _returnvalue (`self.GetNumPlayers` (`GameplayStatics.GetGameMode`)))
      (bind _outactors (`GameplayStatics.GetAllActorsOfClass` "/Game/Actors/Player/SushiPlayer_BP.SushiPlayer_BP_C"))
      (for _array_element _outactors
        (bind _returnvalue_2 (`GameplayStatics.GetActorOfClass` "/Script/Engine.PlayerStart"))
        (bind _returnvalue_3 (+ (`self.ActualRotation`) (/ 360.0 (`KismetMathLibrary.Conv_IntToDouble` _returnvalue))))
        (bind _returnvalue_4 (`self.K2_GetActorLocation` _returnvalue_2))
        (bind _z (.z _returnvalue_4))
        (bind _returnvalue_5 (+ (* (`KismetMathLibrary.GetForwardVector` (`KismetMathLibrary.MakeRotator` 0.0 0.0 _returnvalue_3)) (`KismetMathLibrary.Distance2D` (`KismetMathLibrary.Conv_VectorToVector2D` _returnvalue_4))) (`KismetMathLibrary.MakeVector` 0.0 0.0 _z)))
        (`self.K2_SetActorLocation` _array_element _returnvalue_5 false false)
        (`self.K2_SetActorRotation` _array_element (`KismetMathLibrary.FindLookAtRotation` _returnvalue_5 (`KismetMathLibrary.MakeVector` 0.0 0.0 _z)) false)
        (set `self.ActualRotation` _returnvalue_3)))))

(fn `UserConstructionScript`)